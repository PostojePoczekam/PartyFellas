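; Melon pickup that descends from high above toward a point just over the world origin and equips itself on the Fella that touches it.
; While Can is true, Tick eases the mesh toward that point with a delta-time lerp and spins it by a fixed yaw step per frame.
; Overlap with a Fella calls EquipMelon, returns the mesh to its high position and halts motion until Reset re-enables it.
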(event OnComponentBeginOverlap(StaticMeshComponent)
  (params (OverlappedComponent :type Primitive%20Component%20Object%20Reference) (OtherActor :type Actor%20Object%20Reference) (OtherComp :type Primitive%20Component%20Object%20Reference) (OtherBodyIndex :type Integer) (bFromSweep :type Boolean) (SweepResult :type Hit%20Result%20Structure%20%28by%20ref%29))
  (bind _asfella (Utilities|Casting|CastToFella OtherActor))
  (Default|EquipMelon _asfella)
  (Transformation|SetWorldLocation (Variables|Debug|GetStaticMeshComponent) "0, 0,6000.000000" false false)
  (Variables|Default|Setcan false))

(event Custom|Reset
  (Transformation|SetWorldLocation (Variables|Debug|GetStaticMeshComponent) "0, 0,6000.000000" false false)
  (Variables|Default|Setcan true))

(event EventBeginPlay)

(event EventTick
  (params (DeltaSeconds :type Float%20%28single-precision%29))
  (bind _staticmeshcomponent (Variables|Debug|GetStaticMeshComponent))
  (if (Variables|Default|Getcan)
    (Transformation|SetWorldLocation _staticmeshcomponent (Math|Vector|Lerp(Vector) (Transformation|GetWorldLocation _staticmeshcomponent) (Math|Vector|MakeVector 0.0 0.0 1e+02) (/ DeltaSeconds 1e+01)) false false)
    (Transformation|AddWorldRotation (Variables|Debug|GetStaticMeshComponent) (Math|Rotator|MakeRotator 0.0 0.0 1.0) false false)))

(fn ConstructionScript)