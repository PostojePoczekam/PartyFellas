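; PillSpawner is an actor that periodically launches Pile projectiles at random Fella characters while active.
; Start caches every Fella flagged as Declared, resets the timer and picks a random first delay; Stop halts spawning.
; Tick counts up to the delay, spawns a Pile at the spawner, aims its ProjectileMovement horizontally toward a random cached Fella at fixed speed, then rerolls the interval.
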(event Custom|Start
  (bind _fellas (Variables|Default|Getfellas))
  (Variables|Default|Setseed (Math|Random|RandomFloatinRange 6.0 12.0))
  (Utilities|Array|Clear _fellas)
  (bind _outactors (Actor|GetAllActorsOfClass "/Game/Blueprints/Fella.Fella_C"))
  (for _array_element _outactors
    (if (Variables|/Game/Blueprints/Fella.Fella_C|Getdeclared _array_element)
      (Utilities|Array|Add _fellas _array_element)))
  (Variables|Default|Settimer 0.0)
  (Variables|Default|Setcan true))

(event Custom|Stop
  (Variables|Default|Settimer 0.0)
  (Variables|Default|Setcan false))

(event Collision|EventActorBeginOverlap
  (params (OtherActor :type Actor%20Object%20Reference)))

(event EventTick
  (params (DeltaSeconds :type Float%20%28single-precision%29))
  (bind _fellas (Variables|Default|Getfellas))
  (if (Variables|Default|Getcan)
    (bind _output_get (Variables|Default|Settimer (+ DeltaSeconds (Variables|Default|Gettimer))))
    (if (> _output_get (Variables|Default|Getseed))
      (Variables|Default|Settimer 0.0)
      (bind _returnvalue (Game|SpawnActorfromClass "/Game/Blueprints/Pile.Pile_C" (Transformation|GetActorTransform) "Undefined" 0 0))
      (Game|Components|ProjectileMovement|SetVelocityinLocalSpace (Variables|/Game/Blueprints/Pile.Pile_C|GetProjectileMovement _returnvalue) (Math|Vector|MakeVector (.x (* (Math|Vector|NegateVector (Math|Vector|Normalize (- (Transformation|GetWorldLocation (Variables|/Game/Blueprints/Pile.Pile_C|GetDefaultSceneRoot _returnvalue)) (Transformation|GetWorldLocation (Variables|/Script/Engine.Character|GetCapsuleComponent (Utilities|Array|Get(acopy) _fellas (Math|Random|RandomIntegerinRange 0 (- (Utilities|Array|Length _fellas) 1)))))))) 8e+02)) (.y (* (Math|Vector|NegateVector (Math|Vector|Normalize (- (Transformation|GetWorldLocation (Variables|/Game/Blueprints/Pile.Pile_C|GetDefaultSceneRoot _returnvalue)) (Transformation|GetWorldLocation (Variables|/Script/Engine.Character|GetCapsuleComponent (Utilities|Array|Get(acopy) _fellas (Math|Random|RandomIntegerinRange 0 (- (Utilities|Array|Length _fellas) 1)))))))) 8e+02)) 0.0))
      (Variables|Default|Setseed (Math|Random|RandomFloatinRange 5.0 2e+01)))))

(fn ConstructionScript)