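; Fella is a gamepad-driven, twin-stick multiplayer character with physics-simulated upper body, joined by button press, which starts Timers once multiple players declare.
; While alive and started, Tick feeds sticks into movement, facing and automatic firing.
; Shots launch the character backwards: the default cannon escalates its ball's Level per shot, while a melon grants a temporary spread-fire minigun.
; Damage drives a material Health parameter and kills at a threshold.
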(event Custom|ReloadMinigun
  ;[1 1 1] Weapon Reloading
  (Utilities|FlowControl|Delay 0.01)
  (Variables|Default|SetminigunReloaded true))

(event Custom|ReloadCannon
  ;[1 1 1] Weapon Reloading
  (Utilities|FlowControl|Delay 2.0)
  (Variables|Default|SetcannonReloaded true)
  (Rendering|SetVisibility (Variables|Default|GetBomb) true false))

(event Custom|DealDamage
  (params (damage :type Float%20%28single-precision%29))
  (Variables|Default|Setdamage (+ damage (Variables|Default|Getdamage)))
  (Rendering|Material|SetScalarParameterValueonMaterials (Variables|Character|GetMesh) "Health" (Variables|Default|Getdamage))
  (Game|SpawnActorfromClass "/Game/Blueprints/Hit.Hit_C" (Transformation|GetActorTransform) "Undefined" 0 0)
  (if (>= (Variables|Default|Getdamage) 1.0)
    (Variables|Default|Setalive false)))

(event Custom|EquipMelon
  (Rendering|SetVisibility (Variables|Default|GetMelon) true false)
  (Variables|Default|Setweapon "NewEnumerator1")
  (Utilities|FlowControl|Delay 5.0)
  (CallFunction|EquipBomb))

(event Custom|EquipBomb
  (Rendering|SetVisibility (Variables|Default|GetMelon) false false)
  (Variables|Default|Setweapon "NewEnumerator2"))

(event EventBeginPlay
  (Class|SkeletalMeshComponent|SetAllBodiesBelowSimulatePhysics (Variables|Character|GetMesh) (Utilities|Name|MakeLiteralName "bone_Spine2") true true))

(event EventTick
  (params (DeltaSeconds :type Float%20%28single-precision%29))
  (bind _bomb (Variables|Default|GetBomb))
  (bind _runsmoke (Variables|Default|GetRunSmoke))
  (if (and (Variables|Default|Getalive) (Variables|Default|Getstarted))
    (Utilities|FlowControl|Sequence
      (:then_0
        ;[1 1 1] Handle Input
        (Variables|Default|SetmoveVector (Math|Vector|MakeVector (Input|AxisValues|GetLeftVertical) (Input|AxisValues|GetLeftHorizontal) 0.0))
        (Variables|Default|SetaimVector (Math|Vector|MakeVector (Input|AxisValues|GetRightVertical) (Input|AxisValues|GetRightHorizontal) 0.0)))
      (:then_1
        ;[1 1 1] Move and rotate
        (CallFunction|Move (Variables|Default|GetmoveVector))
        (if (> (Math|Vector|VectorLengthSquared (Variables|Default|GetaimVector)) 0.1)
          (CallFunction|Rotate (Variables|Default|GetaimVector))
          (elif (> (Math|Vector|VectorLengthSquared (Variables|Default|GetmoveVector)) 0.1)
            (CallFunction|Rotate (Variables|Default|GetmoveVector)))))
      (:then_2
        (if (> (Math|Vector|VectorLengthSquared (Variables|Default|GetaimVector)) 0.1)
          (CallFunction|Shoot)))
      (:then_4
        (Transformation|SetRelativeLocation _bomb (Math|Vector|RotateVector (Variables|/Script/Engine.SceneComponent|GetRelativeLocation _bomb) (Math|Rotator|MakeRotator 0.0 0.0 1.0)) false false)
        (Variables|Default|SetammoRotation (+ (Variables|Default|GetammoRotation) DeltaSeconds)))
      (:then_5
        (if (> (Math|Vector|VectorLengthSquared (Variables|Default|GetmoveVector)) 0.1)
          (Components|Activation|SetActive _runsmoke true false)
          (else
            (Components|Activation|SetActive _runsmoke false false)))))))

(event Input|GamepadEvents|GamepadFaceButtonBottom
  (params (Key :type Key%20Structure))
  (:Pressed
    (if (Variables|Default|Getalive)
      (Character|Jump)
      (elif (not (Variables|Default|Getstarted))
        (Variables|Default|Setalive true)
        (Transformation|SetWorldLocation (Variables|Collision|GetCapsuleComponent) (Variables|Default|Getspawn) false false)
        (bind _output_get (Variables|Default|Setdamage 0.0))
        (Rendering|Material|SetScalarParameterValueonMaterials (Variables|Character|GetMesh) "Health" _output_get)
        (Variables|Default|Setlevel 0.0)
        (CallFunction|EquipBomb)
        (Variables|Default|Setstarted false)
        (Variables|Default|Setdeclared true)
        (Variables|Default|Setpcount 0)
        (bind _outactors (Actor|GetAllActorsOfClass "Fella_C"))
        (for _array_element _outactors
          (if (Variables|Fella_C|Getdeclared _array_element)
            (bind _result (Math|Integer|IncrementInt (Variables|Default|Getpcount))
              (:%20%20
                (Variables|Default|Setpcount _result)))))
        (bind _outactors_2 (Actor|GetAllActorsOfClass "/Game/UI_Start.UI_Start_C"))
        (for _array_element_2 _outactors_2
          (Actor|DestroyActor _array_element_2))
        (if (> (Variables|Default|Getpcount) 1)
          (bind _outactors_3 (Actor|GetAllActorsOfClass "/Game/Blueprints/Timer.Timer_C"))
          (for _array_element_3 _outactors_3
            (Default|Start _array_element_3)))))))

(fn ConstructionScript)

(fn Move
  (params (direction :type Vector))
  (Class|PawnMovementComponent|AddInputVector (Variables|Character|GetCharacterMovement) direction false))

(fn ShootMinigun
  (bind _aimvector (Variables|Default|GetaimVector))
  (bind _returnvalue (Math|Vector|Normalize _aimvector))
  (if (Variables|Default|GetminigunReloaded)
    (bind _returnvalue_2 (Game|SpawnActorfromClass "/Game/Blueprints/Bullet.Bullet_C" (Math|Transform|MakeTransform (+ (Transformation|GetActorLocation) (* _returnvalue 50)) "0, 0, 0" "1,1,1") "Undefined" 0 0))
    (Utilities|IsValid (Variables|/Game/Blueprints/Bullet.Bullet_C|GetProjectileMovement _returnvalue_2)
      (:Is%20Valid
        (Variables|/Script/Engine.MovementComponent|SetVelocity (Variables|/Game/Blueprints/Bullet.Bullet_C|GetProjectileMovement _returnvalue_2) (* (Math|Vector|RotateVector _returnvalue (Math|Rotator|MakeRotator (Math|Random|RandomFloatinRange -5.0 5.0) (Math|Random|RandomFloatinRange -5.0 5.0) (Math|Random|RandomFloatinRange -5.0 5.0))) 3e+03))
        (Variables|Default|SetminigunReloaded false)
        (CallFunction|ReloadMinigun)
        (Character|LaunchCharacter (* (Math|Vector|NegateVector _returnvalue) 4e+02) true false)
        (Game|SpawnActorfromClass "/Game/Blueprints/Blink.Blink_C" (Transformation|GetActorTransform) "Undefined" 0 0)))))

(fn Shoot
  (switch Utilities|FlowControl|Switch|SwitchonWeapon (Variables|Default|Getweapon)
    (:NewEnumerator1
      (CallFunction|ShootMinigun))
    (:NewEnumerator2
      (CallFunction|ShootCannon))))

(fn ShootCannon
  (bind _aimvector (Variables|Default|GetaimVector))
  (bind _returnvalue (Math|Vector|Normalize _aimvector))
  (if (Variables|Default|GetcannonReloaded)
    (bind _returnvalue_2 (Game|SpawnActorfromClass "/Game/Blueprints/CannonBall.CannonBall_C" (Math|Transform|MakeTransform (+ (Transformation|GetActorLocation) (* _returnvalue 50)) "0, 0, 0" "1,1,1") "Undefined" 0 0))
    (Variables|Default|SetcannonReloaded false)
    (CallFunction|ReloadCannon)
    (Character|LaunchCharacter (* (Math|Vector|NegateVector _returnvalue) 2e+03) true false)
    (Variables|Default|Setlevel (+ (Variables|Default|Getlevel) 0.1))
    (Variables|/Game/Blueprints/CannonBall.CannonBall_C|Setlevel _returnvalue_2 (Variables|Default|Getlevel))
    (Rendering|SetVisibility (Variables|Default|GetBomb) false false)))

(fn Rotate
  (params (lookAtVector :type Vector))
  (bind _returnvalue (Math|Conversions|RotationFromXVector lookAtVector))
  (Transformation|SetWorldRotation (Variables|Character|GetMesh) (Math|Rotator|MakeRotator (.roll _returnvalue) (.pitch _returnvalue) (- (.yaw _returnvalue) 9e+01)) false false))