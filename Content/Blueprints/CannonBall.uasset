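; CannonBall is an area-of-effect actor that damages and knocks back nearby Fella characters, then destroys itself.
; One second after BeginPlay it finds every Fella within a Level-scaled radius, launches each away from its center and deals Level-based damage.
; Meanwhile, Tick lerps the static mesh's scale toward a Level-scaled size, producing a fast expansion that eases out.
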(event EventBeginPlay
  (Utilities|FlowControl|Delay 1.0)
  (bind _outactors (Actor|GetAllActorsOfClass "/Game/Blueprints/Fella.Fella_C"))
  (for _array_element _outactors
    (if (< (Math|Vector|VectorLength (- (Transformation|GetActorLocation _array_element) (Transformation|GetActorLocation))) (+ 2e+02 (* (Variables|Default|Getlevel) 1e+02)))
      (Character|LaunchCharacter _array_element (* (Math|Vector|Normalize (- (Transformation|GetActorLocation _array_element) (Transformation|GetActorLocation))) 3e+03) true false)
      (Default|DealDamage _array_element (+ (Variables|Default|Getlevel) 0.2))))
  (Actor|DestroyActor))

(event Collision|EventActorBeginOverlap
  (params (OtherActor :type Actor%20Object%20Reference)))

(event EventTick
  (params (DeltaSeconds :type Float%20%28single-precision%29))
  (bind _returnvalue (Math|Vector|MakeVector 5e+01 5e+01 5e+01))
  (bind _staticmesh (Variables|Default|GetStaticMesh))
  (Transformation|SetRelativeScale3D _staticmesh (Math|Vector|Lerp(Vector) (Variables|/Script/Engine.SceneComponent|GetRelativeScale3D _staticmesh) (+ _returnvalue (* _returnvalue (Variables|Default|Getlevel))) (* DeltaSeconds 5.0))))

(fn ConstructionScript)