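; Pile is a spinning pickup-style actor that knocks a Fella character away on contact and then disappears.
; Tick rotates its StaticMesh at a constant per-frame rate, independent of delta time.
; On StaticMesh overlap with a Fella, it launches the character directly away from the Pile with a strong, velocity-overriding impulse, then destroys itself.
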(event OnComponentBeginOverlap(StaticMesh)
  (params (OverlappedComponent :type Primitive%20Component%20Object%20Reference) (OtherActor :type Actor%20Object%20Reference) (OtherComp :type Primitive%20Component%20Object%20Reference) (OtherBodyIndex :type Integer) (bFromSweep :type Boolean) (SweepResult :type Hit%20Result%20Structure%20%28by%20ref%29))
  (bind _asfella (Utilities|Casting|CastToFella OtherActor))
  (Character|LaunchCharacter _asfella (* (Math|Vector|Normalize (- (Transformation|GetActorLocation OtherActor) (Transformation|GetActorLocation))) 5000) true true)
  (Actor|DestroyActor))

(event EventBeginPlay)

(event Collision|EventActorBeginOverlap
  (params (OtherActor :type Actor%20Object%20Reference)))

(event EventTick
  (params (DeltaSeconds :type Float%20%28single-precision%29))
  (Transformation|AddWorldRotation (Variables|Default|GetStaticMesh) "1.000000,3.000000,0.300000" false false))

(fn ConstructionScript)