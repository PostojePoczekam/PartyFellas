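; Camera that turns to follow the living Fella actors in the level, which it gathers once at BeginPlay.
; Each tick it eases the camera's rotation toward a point built from FellasCenter's X and Y, using delta time as lerp alpha.
; FellasCenter sums living Fellas' capsule locations and divides by CountFellas, which as written returns at the first living Fella rather than counting all.
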(event EventBeginPlay
  (bind _outactors (Actor|GetAllActorsOfClass "/Game/Blueprints/Fella.Fella_C"))
  (Variables|Default|Setfellas _outactors))

(event EventTick
  (params (DeltaSeconds :type Float%20%28single-precision%29))
  (bind _target (CallFunction|FellasCenter))
  (Transformation|SetWorldRotation (Variables|CameraActor|GetCameraComponent) (Math|Rotator|Lerp(Rotator) (Transformation|GetWorldRotation (Variables|CameraActor|GetCameraComponent)) (Math|Rotator|FindLookatRotation (Transformation|GetWorldLocation (Variables|CameraActor|GetCameraComponent)) (Math|Vector|MakeVector (.x _target) (.y _target) 0.0)) DeltaSeconds true) false false))

(fn ConstructionScript)

(fn FellasCenter
  (for _array_element (Variables|Default|Getfellas)
    (if (Variables|/Game/Blueprints/Fella.Fella_C|Getalive _array_element)
      (LocalVariables|Setcenter (+ (LocalVariables|Getcenter) (Transformation|GetWorldLocation (Variables|/Script/Engine.Character|GetCapsuleComponent _array_element))))))
  (bind _fellascount (CallFunction|CountFellas))
  (return (/ (LocalVariables|Getcenter) _fellascount)))

(fn CountFellas
  (for _array_element (Variables|Default|Getfellas)
    (if (Variables|/Game/Blueprints/Fella.Fella_C|Getalive _array_element)
      (bind _output_get (LocalVariables|Setcount (+ (LocalVariables|Getcount) 1)))
      (return (+ _output_get 1)))))