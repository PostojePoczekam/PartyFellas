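; Timer is a countdown actor that starts a round of the game.
; Its Start event flashes 3, 2, 1 and GO in sequence using visibility toggles and delays.
; It then marks every Fella as started, teleports undeclared ones to a fixed point below the world origin, resets every AscendingMelon, hides GO and starts every PillSpawner.
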(event Custom|Start
  (bind _2 (Variables|Default|Get2))
  (bind _1 (Variables|Default|Get1))
  (bind _go (Variables|Default|GetGO))
  (bind _3 (Variables|Default|Get3))
  (Rendering|ToggleVisibility _3 false)
  (Utilities|FlowControl|Delay 1.5)
  (Rendering|ToggleVisibility _3 false)
  (Rendering|ToggleVisibility _2 false)
  (Utilities|FlowControl|Delay 1.5)
  (Rendering|ToggleVisibility _2 false)
  (Rendering|ToggleVisibility _1 false)
  (Utilities|FlowControl|Delay 1.5)
  (Rendering|ToggleVisibility _1 false)
  (Rendering|ToggleVisibility _go false)
  (Utilities|FlowControl|Delay 1.0)
  (bind _outactors (Actor|GetAllActorsOfClass "/Game/Blueprints/Fella.Fella_C"))
  (for _array_element _outactors
    (Variables|/Game/Blueprints/Fella.Fella_C|Setstarted _array_element true)
    (if (not (Variables|/Game/Blueprints/Fella.Fella_C|Getdeclared _array_element))
      (Transformation|SetWorldLocation (Variables|/Script/Engine.Character|GetCapsuleComponent _array_element) "0, 0,-558.509460" false false)))
  (bind _outactors_2 (Actor|GetAllActorsOfClass "/Game/Blueprints/AscendingMelon.AscendingMelon_C"))
  (for _array_element_2 _outactors_2
    (Default|Reset _array_element_2))
  (Rendering|ToggleVisibility _go false)
  (bind _outactors_3 (Actor|GetAllActorsOfClass "/Game/Blueprints/PillSpawner.PillSpawner_C"))
  (for _array_element_3 _outactors_3
    (Default|Start _array_element_3)))

(event EventBeginPlay)

(event Collision|EventActorBeginOverlap
  (params (OtherActor :type Actor%20Object%20Reference)))

(event EventTick
  (params (DeltaSeconds :type Float%20%28single-precision%29)))

(fn ConstructionScript)